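; Procedural walking leg component that computes one foot's position for its owning character, updated through the Leg Manager.
; Sphere traces find a target ahead along movement input, handling walls and optional ledge perching for non-bipeds.
; When too far from target, the foot requests manager permission, then steps using speed and height curves timed by step length and max speed.
; Stepping positions go to the manager's LegInfo; falling resets them unless midair tracing is enabled.
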(event EventBeginPlay
  (bind _returnvalue (Transformation|GetWorldLocation))
  ;[0 0 0] At start we're setting some variables for later use. The positions are also important to set beforehand, or the Mesh will start out from the world origin and quickly move towards the actor position on start.
  (Variables|Default|SetLeg%20Manager (Actor|GetComponentbyClass (Components|GetOwner) (Variables|LegSettings|GetBP%20Leg%20Manager%20Class)))
  (Variables|Internal|SetFoot%20Position _returnvalue)
  (Variables|Internal|SetPlant%20Start%20Position _returnvalue)
  (bind _output_get (Variables|Default|SetCharacter%20Movement%20Component (Actor|GetComponentbyClass (Components|GetOwner) "/Script/Engine.CharacterMovementComponent")))
  (Variables|/Script/Engine.CharacterMovementComponent|SetRotationRate _output_get (Math|Rotator|MakeRotator 0.0 0.0 (Variables|LegSettings|GetRotation%20Speed)))
  (Variables|Internal|SetCalculatedStepLength (Variables|LegSettings|GetStep%20Length_Walk))
  (Variables|Internal|SetLastMovementspeed (Class|MovementComponent|GetMaxSpeed (Variables|Default|GetCharacter%20Movement%20Component))))

(fn UpdateFoot
  (params (Index :type Integer))
  (bind _returnvalue (Transformation|GetWorldLocation))
  ;[0 0 0] This is our basic loop, which will be called by the Leg-Manager to update the Foot position.
  (Variables|Internal|SetLegCount Index)
  (if (not (AI|Components|NavMovement|IsFalling (Variables|Default|GetCharacter%20Movement%20Component)))
    (CallFunction|UpdateStepLength :!label _label)
    (UpdateFoot|GetFootTargetLocation)
    (UpdateFoot|CheckforReplant)
    (UpdateFoot|TakeFootStep)
    (elif (Variables|LegSettings|GetKeepTracingMidair)
      (goto _label)
      (else
        ;[0 0 0] In case the Character is falling/jumping we will stop all calculations and fallback to default values.
        (Utilities|Array|SetArrayElem (Variables|/Game/Procedural_Walk_BPs/BP_Leg_Manager_V2.BP_Leg_Manager_V2_C|GetLeg_Info (Actor|GetComponentbyClass (Components|GetOwner) (Variables|LegSettings|GetBP%20Leg%20Manager%20Class))) (Variables|Internal|GetLegCount) _returnvalue true)
        (bind _output_get (Variables|Internal|SetFoot%20Position _returnvalue))
        (Variables|Internal|SetNewTarget%20Position _output_get)
        (Variables|Internal|SetIsPlanted true)))))

(fn CheckforReplant
  (Utilities|FlowControl|Sequence
    (:then_0
      ;[0 0 0] Here we check if it's worth replanting the foot. If the lengt between the Foot-Position and the Target-Position is big enough, it will try to replant unless it already is planted. This will remove unnecessary foot movement, and after stopping any movement it will relplant all legs to their base position if they're too far away, which looks and feels much more natural.
      (LocalVariables|SetWant%20To%20Replant (and (Variables|Internal|GetIsPlanted) (> (Math|Vector|VectorLength (- (Variables|Internal|GetFoot%20Position) (Variables|Internal|GetNewTarget%20Position))) (Variables|LegSettings|GetReplantDistance)))))
    (:then_1
      ;[0 0 0] If the Leg wants to replant, it will ask the Leg-Manager for permission. Only after having the leg wanting to replace and the Leg-Manager allowing it, we will set the leg to actually do the replant.
      (LocalVariables|SetDo%20Replant (and (LocalVariables|GetWant%20To%20Replant) (Default|CanLegUnplant (Variables|Default|GetLeg%20Manager) self))))
    (:then_2
      ;[0 0 0] If we do replant the leg, we set the leg as unplanted, set the current Foot-Position as the Plant-Start-Position for later use, and reset the Time-Since-Unplanted.
      (if (LocalVariables|GetDo%20Replant)
        (Utilities|FlowControl|Sequence
          (:then_0
            (Variables|Internal|SetIsPlanted false))
          (:then_1
            (Variables|Internal|SetPlant%20Start%20Position (Variables|Internal|GetFoot%20Position)))
          (:then_2
            (Variables|Internal|SetTimeSinceUnplanted 0.0)))))))

(fn GetFootTargetLocation
  (bind _returnvalue (Components|GetOwner))
  (bind _returnvalue_2 (Transformation|GetWorldLocation))
  (bind _returnvalue_3 (Transformation|GetActorLocation _returnvalue))
  (Utilities|FlowControl|Sequence
    (:then_0
      ;[0 0 0 0.5] First we do a precheck Sphere-trace in case our foot is physically placed too far away from the main Collision-Caspsule of our character and there is a another object in between. Because in that case the following traces would not work. So we trace between our characters location and the foot location for a hit. If we hit something, we tell the next trace to use thise new position slightly infront of whatever we hit via the "VirtualComponentPosition". If we don't hit anything we're safe and can just use the default position. If we do hit something, we get the normal of whatever we hit which will give us the direction perpendicular (90°) to that surface and we draw it out to get the position slightly in front of that surface to use as our new position.
      (bind (_outhit _returnvalue_4) (Collision|SphereTraceByChannel (Math|Vector|MakeVector (.x _returnvalue_3) (.y _returnvalue_3) (+ (.z _returnvalue_3) (Variables|LegSettings|GetWall%20Trace%20Height))) (Math|Vector|MakeVector (.x _returnvalue_2) (.y _returnvalue_2) (+ (.z (Transformation|GetActorLocation (Components|GetOwner))) (Variables|LegSettings|GetWall%20Trace%20Height))) (Variables|LegSettings|GetWallTraceRadius) "TraceTypeQuery1" (Variables|LegSettings|GetTrace%20Complex) 0 (Variables|LegSettings|GetDraw%20Debug%20Type) true "(R=0.985715,G=0.000000,B=1.000000,A=1.000000)"))
      (if _returnvalue_4
        (Variables|Internal|SetVirtualComponentPosition (+ (Math|Vector|MakeVector (.x (.location _outhit)) (.y (.location _outhit)) (.z (Transformation|GetWorldLocation))) (* (.normal _outhit) 5.0)))
        (else
          (Variables|Internal|SetVirtualComponentPosition (Transformation|GetWorldLocation)))))
    (:then_1
      ;[0 0 0] Then we set our InputVector. It's determined by the direction our Actor is traveling.
      (Variables|Internal|SetInput%20Vector (Math|Vector|Normalize (Pawn|Components|PawnMovement|GetLastInputVector (Variables|Default|GetCharacter%20Movement%20Component)))))
    (:then_2
      ;[0 0 0] Then we get the Up-Vector of the Owner to which this component is attached to (so we get the Actors relative version of "up") and multiply that by the Trace-Height. This gives us the elevation we need. Very important for traces is to not forget to add the current world location. So we add the Current World location of our component to the elevation. And now to actually find the future position, we take the InputVector and multiply it by the CalculatedStepLength, which determines the length the foot will travel, and add it as well. This finally results in our Trace starting position.
      (LocalVariables|SetRay%20Start (+ (+ (* (Transformation|GetActorUpVector (Components|GetOwner)) (Variables|LegSettings|GetTrace%20Height)) (Variables|Internal|GetVirtualComponentPosition)) (* (Variables|Internal|GetInput%20Vector) (Variables|Internal|GetCalculatedStepLength)))))
    (:then_3
      ;[0 0 0] Now we do the same thing but negate the UpVector to get whatever the Actor considers "down". To reach far enough down we multiply the TraceHeight by a NegativeTraceHeightMultiplier, which should be atleast 2 for it to trace the same distance up and down. This will give us the end position of our trace.
      (LocalVariables|SetRay%20End (+ (+ (* (Math|Vector|NegateVector (Transformation|GetActorUpVector (Components|GetOwner))) (* (Variables|LegSettings|GetTrace%20Height) (Variables|LegSettings|GetNegativeTraceHeightMultiplier))) (Variables|Internal|GetVirtualComponentPosition)) (* (Variables|Internal|GetInput%20Vector) (Variables|Internal|GetCalculatedStepLength)))))
    (:then_4
      ;[0 0 0] Then we plug the RayStart and RayEnd into a Spheretrace. If it does hit something, we grab that ImpactPoint and use it as the TargetPosition. If we don't hit something we try a Fallback-Trace which does the same to look for a surface beneath the charcter to "Perch" on, unless it's a Biped, in that case we skip that and just use the default component location.
      (bind (_outhit_2 _returnvalue_5) (Collision|SphereTraceByChannel (LocalVariables|GetRay%20Start) (LocalVariables|GetRay%20End) (Variables|LegSettings|GetSphereTraceRadius) "TraceTypeQuery1" (Variables|LegSettings|GetTrace%20Complex) 0 (Variables|LegSettings|GetDraw%20Debug%20Type)))
      (if _returnvalue_5
        (Variables|Internal|SetCalculatedTargetPosition (.ImpactPoint (Collision|BreakHitResult _outhit_2)))
        (else
          (|SphereTrace2))))
    (:then_5
      ;[0 0 0 0.5] To prevent the leg teleporting during transition in case a new target position has been applied that is much further away (from one ledge to another), we use and interpolation to smooth the transition.
      (bind _output_get (Variables|Internal|SetNewTarget%20Position (Math|Interpolation|VInterpTo (Variables|Internal|GetOldTarget%20Position) (Variables|Internal|GetCalculatedTargetPosition) (Utilities|Time|GetWorldDeltaSeconds) 15.0)))
      (Variables|Internal|SetOldTarget%20Position _output_get))
    (:then_6
      ;[0 0 0] This is to visualize the calculated positions during gameplay.
      (|Visualization))))

(fn TakeFootStep
  (if (Variables|Internal|GetIsPlanted)
    (return)
    (else
      (Utilities|FlowControl|Sequence
        (:then_0
          ;[0 0 0] Get the CalculatedStepLength and divide it by the Character_BP's current max movement speed (which is expressed in cm/s), this will give us the time it takes to make 1 step and will determine how fast the "animation" plays.
          (Variables|Internal|SetStepTime (/ (Variables|Internal|GetCalculatedStepLength) (Class|MovementComponent|GetMaxSpeed (Variables|Default|GetCharacter%20Movement%20Component)))))
        (:then_1
          ;[0 0 0] By dividing the TimeSinceUnplanted by the StepTime we can track the progress of the step.
          (Variables|Internal|SetPercentage%20Replanted (/ (Variables|Internal|GetTimeSinceUnplanted) (Variables|Internal|GetStepTime))))
        (:then_2
          ;[0 0 0] Now we lerp from the Plant-Start-Position towards the traced Target-Position and set it as the Foot-Position. Lerp chooses a point between A and B depending on the Alpha value (which goes from 0 to 1), so using the current step progression expressed in the Percentage-Replanted it will return the corresponding value of the curve. The curves give us better control of the actual foot movement. So we use the same method to get the height of the foot during replanting. Change the Step-Height to change the amount the foot will be lifted.
          (Variables|Internal|SetFoot%20Position (+ (Math|Vector|Lerp(Vector) (Variables|Internal|GetPlant%20Start%20Position) (Variables|Internal|GetNewTarget%20Position) (Math|Curves|GetFloatValue (LocalVariables|GetReplant%20Speed%20Curve) (Variables|Internal|GetPercentage%20Replanted))) (* (Transformation|GetActorUpVector (Components|GetOwner)) (- (* (Math|Curves|GetFloatValue (LocalVariables|GetReplant%20Height%20Curve) (Variables|Internal|GetPercentage%20Replanted)) (Variables|LegSettings|GetStep%20Height)) (Variables|LegSettings|GetFoot%20Offset)))))
          (Utilities|Array|SetArrayElem (Variables|/Game/Procedural_Walk_BPs/BP_Leg_Manager_V2.BP_Leg_Manager_V2_C|GetLeg_Info (Actor|GetComponentbyClass (Components|GetOwner) (Variables|LegSettings|GetBP%20Leg%20Manager%20Class))) (Variables|Internal|GetLegCount) (Variables|Internal|GetFoot%20Position) true))
        (:then_3
          ;[0 0 0] After that we will Add the current runtime to the TimeSinceUnplanted and set it as the new TimeSinceUnplanted. This way it will count up towards the StepTime. As soon as the TimeSinceUnplanted is equal or greater than the StepTime we will consider the step finished and we will let the Leg-Manager know.
          (bind _output_get (Variables|Internal|SetTimeSinceUnplanted (+ (Variables|Internal|GetTimeSinceUnplanted) (Utilities|Time|GetWorldDeltaSeconds))))
          (Variables|Internal|SetIsPlanted (>= _output_get (Variables|Internal|GetStepTime))))))))

(fn UpdateStepLength
  ;[0 0 0 0.5] For a better experience our Actor should have different Steplengths depending on if it's walking or running. Here we determine if the movement state has changed in speed. Generally we start out with the Walk-Speed and see if the speed has increased in relation to the speed we had on the last tick. If the speed hasn't changed we continue as normal.
  (if (== (Variables|Internal|GetLastMovementspeed) (Class|MovementComponent|GetMaxSpeed (Variables|Default|GetCharacter%20Movement%20Component)))
    _
    (else
      ;[0 0 0 0.5] Don't forget to set the LastMovementSpeed from the current MaxSpeed of the MovementComponent for the next tick.
      (Variables|Internal|SetCalculatedStepLength (Math|Interpolation|FInterpTo (Variables|Internal|GetCalculatedStepLength) (Math|Float|SelectFloat (Variables|LegSettings|GetStep%20Length_Run) (Variables|LegSettings|GetStep%20Length_Walk) (< (Variables|Internal|GetLastMovementspeed) (Class|MovementComponent|GetMaxSpeed (Variables|Default|GetCharacter%20Movement%20Component)))) (Utilities|Time|GetWorldDeltaSeconds) 1.0))))
  (Variables|Internal|SetLastMovementspeed (Class|MovementComponent|GetMaxSpeed (Variables|Default|GetCharacter%20Movement%20Component))))