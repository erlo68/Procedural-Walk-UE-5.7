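; Leg manager component for procedural walking that updates its owner's BP_Leg components and decides when each may lift.
; BeginPlay sorts legs by the L/R and trailing digit in their names into one array alternating left and right, starting left.
; Tick calls UpdateFoot on each leg with its index.
; CanLegUnplant requires the leg and one neighbor to be planted: the opposite leg for the front pair, otherwise the leg ahead.
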(event EventTick
  (params (DeltaSeconds :type Float%20%28single-precision%29))
  ;[0 0 0] On each Tick go trough the feet array and call their update function.
  (for (_array_element _array_index) (Variables|Default|GetFeet)
    (Default|UpdateFoot _array_element _array_index)))

(event EventBeginPlay
  ;[0 0 0] On Begin Play, grab all BP_Leg instances attached to the owner and put them in an array.
  (for _array_element (Actor|GetComponentsByClass (Components|GetOwner) (Variables|ManagerSettings|GetBP_Leg_Class))
    (Utilities|Array|Add (Variables|Default|GetFeet) _array_element))
  ;[0 0 0] This is only neccessary since the sorting method of Blueprint-Components is unreliable. Here, we go trough the Array and sort them into a different Array depending on wether it's a left or a right leg. At the same time they're being put into the correct order. Important to know is that the original component must not have an "L" or "R" in it's name besides the left/right designation. This is why they should be called "Foot_L1" instead of "Leg_L1" or something like that.
  (for _array_element_2 (Variables|Default|GetFeet)
    (if (Utilities|String|Contains (Utilities|GetObjectName _array_element_2) "L" false true)
      (Utilities|Array|SetArrayElem (Variables|Default|GetFeet_L) (- (Math|Conversions|ToInteger(Byte) (Utilities|String|Right (Utilities|GetObjectName _array_element_2) 1)) 1) _array_element_2 true)
      (else
        (Utilities|Array|SetArrayElem (Variables|Default|GetFeet_R) (- (Math|Conversions|ToInteger(Byte) (Utilities|String|Right (Utilities|GetObjectName _array_element_2) 1)) 1) _array_element_2 true))))
  ;[0 0 0] After sorting them by left and right, we put them back into the original array. We're flip-floping between the arrays to always have the opposing leg in the next line. This way we can easily go trough the array and have the legs be in the correct order so it will call R1, L1, R2, L2 and so on. This is important for later when we check wether the leg is allowed to unplant.
  (Variables|Default|SetCount_R 0)
  (Variables|Default|SetCount_L 0)
  (for (_ _array_index) (Variables|Default|GetFeet)
    (if (> (Math|Integer|%(Integer) _array_index 2) 0)
      (Utilities|Array|SetArrayElem (Variables|Default|GetFeet) _array_index (Utilities|Array|Get(acopy) (Variables|Default|GetFeet_R) (Variables|Default|GetCount_R)) true)
      (Variables|Default|SetCount_R (+ (Variables|Default|GetCount_R) 1))
      (else
        (Utilities|Array|SetArrayElem (Variables|Default|GetFeet) _array_index (Utilities|Array|Get(acopy) (Variables|Default|GetFeet_L) (Variables|Default|GetCount_L)) true)
        (Variables|Default|SetCount_L (+ (Variables|Default|GetCount_L) 1))))))

(fn CanLegUnplant
  (params (Leg :type BP%20Leg%20V2%20Object%20Reference))
  (bind _legcount (Variables|/Game/Procedural_Walk_BPs/BP_Leg_V2.BP_Leg_V2_C|GetLegCount Leg))
  ;[0 0 0] If it's the first leg, only check the physically opposite leg.
  (if (== _legcount 0)
    (if (and (Variables|/Game/Procedural_Walk_BPs/BP_Leg_V2.BP_Leg_V2_C|GetIsPlanted (Utilities|Array|Get(acopy) (Variables|Default|GetFeet) 1)) (Variables|/Game/Procedural_Walk_BPs/BP_Leg_V2.BP_Leg_V2_C|GetIsPlanted Leg))
      (return true)
      (else
        (return false)))
    (else
      ;[0 0 0] If it's the second leg, only check the first leg.
      (if (== _legcount 1)
        (if (and (Variables|/Game/Procedural_Walk_BPs/BP_Leg_V2.BP_Leg_V2_C|GetIsPlanted (Utilities|Array|Get(acopy) (Variables|Default|GetFeet))) (Variables|/Game/Procedural_Walk_BPs/BP_Leg_V2.BP_Leg_V2_C|GetIsPlanted Leg))
          (return true)
          (else
            (return false)))
        (else
          ;[0 0 0] If it's neither the first nor the second leg, check the leg physically in front of this one.
          (if (and (Variables|/Game/Procedural_Walk_BPs/BP_Leg_V2.BP_Leg_V2_C|GetIsPlanted Leg) (Variables|/Game/Procedural_Walk_BPs/BP_Leg_V2.BP_Leg_V2_C|GetIsPlanted (Utilities|Array|Get(acopy) (Variables|Default|GetFeet) (- _legcount 2))))
            (return true)
            (else
              (return false))))))))